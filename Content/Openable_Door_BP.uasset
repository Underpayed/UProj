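; Openable door actor that swings open and closed when its OpenDoor component fires open and close events.
; It stores its starting rotation at BeginPlay, then a timeline drives a yaw angle combined with that rotation.
; Closing plays the same timeline in reverse, and a timeline event track plays a door lock sound at the actor's location.
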(event `self.ReceiveBeginPlay`
  (set `self.InitialRotation` (`self.K2_GetActorRotation`)))

(event `self.OpenDoor.OnOpen`
  (bind (_direction _openangle) (`Timeline|TimeLineSwing` :!label _label)
    (:`Update`
      (`self.K2_SetActorRotation` (`KismetMathLibrary.ComposeRotators` (`KismetMathLibrary.MakeRotator` 0.0 0.0 _openangle) (`self.InitialRotation`))))
    (:`SoundDoorLock`
      (`GameplayStatics.PlaySoundAtLocation` "/Game/Audio/door-lock.door-lock" (`self.K2_GetActorLocation`)))))

(event `self.OpenDoor.OnClose`
  (goto _label :!via `Reverse`))

(fn `UserConstructionScript`)